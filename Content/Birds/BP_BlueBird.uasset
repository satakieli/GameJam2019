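; BP_BlueBird is a bird projectile that splits into three by spawning two copies of itself shortly after launch.
; The BirdLaunched event waits briefly, then spawns one copy on each side, offset along the player rotation's right vector.
; Each copy's mesh gets the launch velocity, rotated by opposite angles around the player's up vector, and simulates physics.
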(event EventBirdLaunched
  (params (Velocity :type Vector :default "0, 0, 0") (Player%20Rot :type Rotator :default "0, 0, 0"))
  (bind _returnvalue (Transformation|GetActorTransform))
  (bind _returnvalue_2 (Math|Vector|GetUpVector Player%20Rot))
  (bind _returnvalue_3 (Math|Vector|GetRightVector Player%20Rot))
  (bind _distance (Variables|Default|GetDistance))
  (bind _returnvalue_4 (* _returnvalue_3 _distance))
  (Utilities|FlowControl|Delay 0.1)
  (Utilities|FlowControl|Sequence
    (:then_0
      (bind _returnvalue_5 (Game|SpawnActorfromClass "BP_BlueBird_C" (Math|Transform|MakeTransform (+ (.location _returnvalue) _returnvalue_4) (.rotation _returnvalue) (.scale _returnvalue)) "AlwaysSpawn" 0 0))
      (Physics|SetPhysicsLinearVelocity (Variables|/Game/Birds/BP_Bird.BP_Bird_C|GetBirdMesh _returnvalue_5) (Math|Vector|RotateVectorAroundAxis Velocity -15.0 _returnvalue_2) false "None")
      (Physics|SetSimulatePhysics (Variables|/Game/Birds/BP_Bird.BP_Bird_C|GetBirdMesh _returnvalue_5) true))
    (:then_1
      (bind _returnvalue_6 (Game|SpawnActorfromClass "BP_BlueBird_C" (Math|Transform|MakeTransform (+ (.location _returnvalue) (* _returnvalue_4 -1.0)) (.rotation _returnvalue) (.scale _returnvalue)) "AlwaysSpawn" 0 0))
      (Physics|SetPhysicsLinearVelocity (Variables|/Game/Birds/BP_Bird.BP_Bird_C|GetBirdMesh _returnvalue_6) (Math|Vector|RotateVectorAroundAxis Velocity 15.0 _returnvalue_2) false "None")
      (Physics|SetSimulatePhysics (Variables|/Game/Birds/BP_Bird.BP_Bird_C|GetBirdMesh _returnvalue_6) true))))

(fn ConstructionScript
  (|CallParentFunction))