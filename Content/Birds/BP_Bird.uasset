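; BP_Bird is a physics-driven bird actor that can be picked up, carried and dropped, with mass override and prototype color tinting.
; Pickup disables mesh physics and attaches the root to the given component.
; Drop restores physics, detaches, then passes mesh velocity and player rotation to BirdLaunched, an empty event here.
; The construction script creates a dynamic material instance to apply BirdColor, standing in for per-bird meshes.
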(event Custom|Bird%20Launched
  (params (Velocity :type Vector) (Player%20Rot :type Rotator)))

(event EventPickup
  (params (AttachTo :type Scene%20Component%20Object%20Reference))
  ;[1 1 1] When the Bird is picked up we disable the Physics and Attach it to the person Picking it up
  (Physics|SetSimulatePhysics (Variables|Default|GetBirdMesh) false)
  (Transformation|AttachComponentToComponent (VehicleSound|GetRootComponent) AttachTo "None" "KeepWorld" "KeepWorld" "KeepWorld" false))

(event EventDrop
  (params (Player%20Rotation :type Rotator :default "0, 0, 0"))
  (bind _birdmesh (Variables|Default|GetBirdMesh))
  ;[1 1 1] Physics Enabled again and Detached from any actor it is attached to
  (Physics|SetSimulatePhysics _birdmesh true)
  (Transformation|DetachFromActor "KeepWorld" "KeepWorld" "KeepWorld")
  (CallFunction|BirdLaunched (Transformation|GetComponentVelocity _birdmesh) Player%20Rotation))

(event EventBeginPlay
  (Class|PrimitiveComponent|SetMassOverrideinKg (Variables|Default|GetBirdMesh) "None" (Variables|Default|GetBird%20Mass) true))

(fn ConstructionScript
  ;[1 1 1] (PROTOTYPE) Create a Material for the Bird Mesh.
  ; In Real Situation we would have a Mesh for each Bird
  (bind _returnvalue (Rendering|Material|CreateDynamicMaterialInstance (Variables|Default|GetBirdMesh) 0 "/Game/Birds/Bird_MatInst.Bird_MatInst" "None" :!class /Script/Engine.PrimitiveComponent))
  (bind _output_get (Variables|Default|SetBird%20Mat _returnvalue))
  (Rendering|Material|SetVectorParameterValue _output_get "Color" (Variables|Default|GetBird%20Color) :!class /Script/Engine.MaterialInstanceDynamic))